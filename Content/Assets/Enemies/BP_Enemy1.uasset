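; BP_Enemy1 is a simple enemy that hops around at random and repeatedly hurts BP_JonCharacter on contact.
; AIMoveTo picks nearby navigable points from BeginPlay, re-chaining only on success, while Tick calls Jump every frame.
; Capsule overlaps set a contact flag that gates a Delay-throttled TakeDamageJon call on Tick, passing zero as its argument.
; AnyDamage reduces Health and enables mesh physics at zero, without stopping movement or attacks.
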(event `self.ReceiveAnyDamage`
  (params (Damage :type "Float (single-precision)") (DamageType :type "DamageType Object Reference") (InstigatedBy :type "Controller Object Reference") (DamageCauser :type "Actor Object Reference"))
  ;[1 1 1] Enemy Health
  (set `self.health` (- (`self.health`) Damage))
  (if (<= (`self.health`) 0.0)
    (`PrimitiveComponent.SetSimulatePhysics` (`self.Mesh`) true)))

(event `JumpToRandomLocation`
  ;[1 1 1] Budget AI
  (bind _randomlocation (`NavigationSystemV1.K2_GetRandomLocationInNavigableRadius` (`self.K2_GetActorLocation`) 40.0 null null))
  (`|AIMoveTo` null _randomlocation self
    (:`OnSuccess`
      (`self.JumpToRandomLocation`))))

(event `self.ReceiveBeginPlay`
  ;[1 1 1] Budget AI
  (`self.JumpToRandomLocation`))

(event `self.Capsule.OnComponentBeginOverlap`
  (params (OverlappedComponent :type "PrimitiveComponent Object Reference") (OtherActor :type "Actor Object Reference") (OtherComp :type "PrimitiveComponent Object Reference") (OtherBodyIndex :type Integer) (bFromSweep :type Boolean) (SweepResult :type "HitResult Structure (by ref)"))
  ;[1 1 1] DamageOvertimeLogic
  (bind _asbp_jon_character (cast `/Game/Blueprints/MainCharacterBP´s/BP_JonCharacter` OtherActor))
  (set `self.PlayerContact` true)
  (set `self.JonRef` _asbp_jon_character))

(event `self.ReceiveTick`
  (params (DeltaSeconds :type "Float (single-precision)"))
  ;[1 1 1] DamageOvertimeLogic
  (`|ExecutionSequence`
    (:`then_0`
      (`self.Jump`))
    (:`then_1`
      (if (`self.PlayerContact`)
        (`KismetSystemLibrary.Delay` (`self.DamageDelay`))
        (`/Game/Blueprints/MainCharacterBP´s/BP_JonCharacter.TakeDamageJon` (`self.JonRef`) 0.0)))))

(event `self.Capsule.OnComponentEndOverlap`
  (params (OverlappedComponent :type "PrimitiveComponent Object Reference") (OtherActor :type "Actor Object Reference") (OtherComp :type "PrimitiveComponent Object Reference") (OtherBodyIndex :type Integer))
  ;[1 1 1] DamageOvertimeLogic
  (cast `/Game/Blueprints/MainCharacterBP´s/BP_JonCharacter` OtherActor)
  (set `self.PlayerContact` false))

(fn `UserConstructionScript`)