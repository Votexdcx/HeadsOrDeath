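; Game mode that scatters red, green and blue crystals across the level at BeginPlay.
; Each color has its own function that gathers that color's spawn point actors and spawns two crystals at randomly picked locations.
; Each used spawn point is removed from the list and destroyed, so crystals of the same color never share a point.
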(event `self.ReceiveBeginPlay`
  (`self.SpawnRedCrystal`)
  (`self.SpawnGreenCrystal`)
  (`self.SpawnBlueCrystal`))

(fn `SpawnBlueCrystal`
  (locals (LocalItemBlue :type "/Game/CrystalSpawns/BP_SpawnPointBlue Object Reference"))
  (bind _outactors (`GameplayStatics.GetAllActorsOfClass` "/Game/CrystalSpawns/BP_SpawnPointBlue.BP_SpawnPointBlue_C"))
  (set `self.Local Blue Spawn  References` _outactors)
  (for _ (range 2)
    (set `local.LocalItemBlue` (`KismetArrayLibrary.Array_Random` (`self.Local Blue Spawn  References`)))
    (`|SpawnActorFromClass` "/Game/machine_gun/CrystalBP/BlueCrystal.BlueCrystal_C" (`KismetMathLibrary.MakeTransform` (`self.K2_GetActorLocation` (`local.LocalItemBlue`))) "AdjustIfPossibleButAlwaysSpawn" "MultiplyWithRoot" null null)
    (`KismetArrayLibrary.Array_RemoveItem` (`self.Local Blue Spawn  References`) (`local.LocalItemBlue`))
    (`self.K2_DestroyActor` (`local.LocalItemBlue`))))

(fn `SpawnGreenCrystal`
  (bind _outactors (`GameplayStatics.GetAllActorsOfClass` "/Game/CrystalSpawns/BP_SpawnPointGreen.BP_SpawnPointGreen_C"))
  (set `self.Green SPawn References` _outactors)
  (for _ (range 2)
    (set `self.Local Item Green` (`KismetArrayLibrary.Array_Random` (`self.Green SPawn References`)))
    (`|SpawnActorFromClass` "/Game/machine_gun/CrystalBP/GreenCrystal.GreenCrystal_C" (`KismetMathLibrary.MakeTransform` (`self.K2_GetActorLocation` (`self.Local Item Green`))) "AdjustIfPossibleButAlwaysSpawn" "MultiplyWithRoot" null null)
    (`KismetArrayLibrary.Array_RemoveItem` (`self.Green SPawn References`) (`self.Local Item Green`))
    (`self.K2_DestroyActor` (`self.Local Item Green`))))

(fn `SpawnRedCrystal`
  (locals (`Local Item Red` :type "/Game/CrystalSpawns/BP_SpawnPointRed Object Reference"))
  (bind _outactors (`GameplayStatics.GetAllActorsOfClass` "/Game/CrystalSpawns/BP_SpawnPointRed.BP_SpawnPointRed_C"))
  (set `self.Red Spawn References` _outactors)
  (for _ (range 2)
    (set `local.Local Item Red` (`KismetArrayLibrary.Array_Random` (`self.Red Spawn References`)))
    (`|SpawnActorFromClass` "/Game/machine_gun/CrystalBP/RedCrystal.RedCrystal_C" (`KismetMathLibrary.MakeTransform` (`self.K2_GetActorLocation` (`local.Local Item Red`))) "AdjustIfPossibleButAlwaysSpawn" "MultiplyWithRoot" null null)
    (`KismetArrayLibrary.Array_RemoveItem` (`self.Red Spawn References`) (`local.Local Item Red`))
    (`self.K2_DestroyActor` (`local.Local Item Red`))))

(fn `UserConstructionScript`)