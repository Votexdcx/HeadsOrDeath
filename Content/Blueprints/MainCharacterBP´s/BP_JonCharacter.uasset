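; BP_JonCharacter is the player character, handling hitscan shooting, health loss and buff selection display.
; IA_Shoot line-traces forward from the camera, applies damage to the hit actor and spawns a muzzle flash on every shot.
; TakeDamageJon subtracts from PlayerHealth and prints a message, with no death check.
; Tick sends BuffSelection to the player controller's buff widget for highlighting; a shooting camera shake is present but unconnected.
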(event `self.ReceiveTick`
  (params (DeltaSeconds :type "Float (single-precision)"))
  (bind _asbp_jon_player_controller (cast `/Game/Blueprints/MainCharacterBP´s/BP_JonPlayerController` (`GameplayStatics.GetPlayerController` 0)))
  (`/Game/UI/BuffDebuffUI/BP_WidgetBuff.BuffHighlight` (`/Game/Blueprints/MainCharacterBP´s/BP_JonPlayerController.BPBuffwidget` _asbp_jon_player_controller) (`self.BuffSelection`)))

(event `EnhancedInput|/Game/FirstPerson/Input/Actions/IA_Shoot`
  (params (ActionValue :type Boolean) (ElapsedSeconds :type "Float (double-precision)") (TriggeredSeconds :type "Float (double-precision)") (InputAction :type "InputAction Object Reference" :default "/Game/FirstPerson/Input/Actions/IA_Shoot.IA_Shoot"))
  (bind (_returnvalue_location _returnvalue_rotation) (`KismetMathLibrary.BreakTransform` (`SceneComponent.K2_GetComponentToWorld` (`self.CameraReal`))))
  (:`Started`
    (`|ExecutionSequence`
      (:`then_0`
        (bind (_outhit _returnvalue) (`KismetSystemLibrary.LineTraceSingle` :`Start` _returnvalue_location :`End` (+ _returnvalue_location (* (`KismetMathLibrary.GetForwardVector` _returnvalue_rotation) 5000.0)) :`TraceChannel` "TraceTypeQuery1" :`DrawDebugType` "ForDuration"))
        (if _returnvalue
          (`GameplayStatics.ApplyDamage` (`.HitActor` (`GameplayStatics.BreakHitResult` _outhit)) (`self.Base Damage`))))
      (:`then_1`
        (`GameplayStatics.SpawnEmitterAttached` "/Game/InfinityBladeEffects/Effects/FX_Monsters/FX_Monster_Chicken/P_ChickenMaster_MuzzleFlash_01.P_ChickenMaster_MuzzleFlash_01" null "Muzzle" (0.0 0.0 0.0) (struct) (0.2 0.2 0.2) "KeepRelativeOffset" true "AutoRelease")))))

(event `TakeDamageJon`
  (params (Damage :type "Float (double-precision)"))
  ;[1 1 1] Player Health System
  (set `self.Player Health` (- (`self.Player Health`) Damage))
  (`KismetSystemLibrary.PrintString` "Player took dmg"))

(fn `UserConstructionScript`)