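; Turret Blueprint that fires at pawns it senses and also carries crystal-spawning logic.
; On seeing BP_JonCharacter, it rotates that character (not itself) along the turret-to-pawn direction, waits briefly, then plays a shoot montage whose notify spawns a projectile at the Arrow.
; SpawnCrystals spawns a given class after a random delay at a navmesh point around a fixed origin.
; A separate function decrements the crystal count.
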(event `SHOOT`
  (bind _arrow (`self.Arrow`))
  (`|PlayMontage` (`self.SK_MESH`) "/Game/ENEMIES/TURRET/TURRET_SHOOT_Montage.TURRET_SHOOT_Montage"
    (:`OnNotifyBegin`
      (`|SpawnActorFromClass` "/Game/Enemy_B1/Enemy_projectilr.Enemy_projectilr_C" (`KismetMathLibrary.MakeTransform` (`SceneComponent.K2_GetComponentLocation` _arrow) (`SceneComponent.K2_GetComponentRotation` _arrow)) "Undefined" "MultiplyWithRoot" null null)
      (`KismetSystemLibrary.Delay` 1.0))))

(event `self.PawnSensing.OnSeePawn`
  (params (Pawn :type "Pawn Object Reference"))
  (bind _asbp_jon_character (cast `/Game/Blueprints/MainCharacterBP´s/BP_JonCharacter` Pawn))
  (`self.K2_SetActorRotation` _asbp_jon_character (`KismetMathLibrary.FindLookAtRotation` (`self.K2_GetActorLocation`) (`self.K2_GetActorLocation` Pawn)) false)
  (`KismetSystemLibrary.Delay` 0.5)
  (`self.SHOOT`))

(event `SpawnCrystals`
  (params (CrysalClass :type "/Game/machine_gun/CrystalBP/Crystal Class Reference"))
  (`KismetSystemLibrary.Delay` (`KismetMathLibrary.RandomFloatInRange` 15.0 20.0))
  (bind _returnvalue (`GameplayStatics.GetActorOfClass` "/Script/NavigationSystem.RecastNavMesh"))
  (bind _output_get (set `self.location` (-682.064697 121.284319 -631.274208)))
  (bind _randomlocation (`NavigationSystemV1.K2_GetRandomLocationInNavigableRadius` _output_get 2000.0 _returnvalue "/Script/AIModule.NavFilter_AIControllerDefault"))
  (`|SpawnActorFromClass` CrysalClass (`KismetMathLibrary.Conv_VectorToTransform` _randomlocation) "AdjustIfPossibleButAlwaysSpawn" "MultiplyWithRoot" null null))

(fn `Subtractnumberofcrystals`
  (set `self.NumberOfCrystals` (- (`self.NumberOfCrystals`) 1)))

(fn `UserConstructionScript`)