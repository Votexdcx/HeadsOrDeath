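; BP_TuRretGreen is the green turret variant, spawning green crystals on BeginPlay and shooting at the player character it sees.
; On sighting BP_JonCharacter, it sets the character's rotation (not its own) along the turret-to-player direction, then calls SHOOT after a short delay.
; Tick polls BP_JonPlayerController and destroys the PawnSensing component once GreenGems reaches zero, which ends detection.
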(event `self.ReceiveBeginPlay`
  (`self.SpawnCrystals` "/Game/machine_gun/CrystalBP/GreenCrystal.GreenCrystal_C"))

(event `self.ReceiveTick`
  (params (DeltaSeconds :type "Float (single-precision)"))
  (`/Engine/EditorBlueprintResources/StandardMacros.IsValid` (`self.PawnSensing`)
    (:`Is Valid`
      (bind _asbp_jon_player_controller (cast `/Game/Blueprints/MainCharacterBP´s/BP_JonPlayerController` (`GameplayStatics.GetPlayerController` 0)))
      (if (== (`/Game/Blueprints/MainCharacterBP´s/BP_JonPlayerController.GreenGems` _asbp_jon_player_controller) 0)
        (`ActorComponent.K2_DestroyComponent` (`self.PawnSensing`))))))

(event `self.PawnSensing.OnSeePawn`
  (params (Pawn :type "Pawn Object Reference"))
  (bind _asbp_jon_character (cast `/Game/Blueprints/MainCharacterBP´s/BP_JonCharacter` Pawn))
  (`self.K2_SetActorRotation` _asbp_jon_character (`KismetMathLibrary.FindLookAtRotation` (`self.K2_GetActorLocation`) (`self.K2_GetActorLocation` Pawn)) false)
  (`KismetSystemLibrary.Delay` 0.5)
  (`self.SHOOT`))

(fn `UserConstructionScript`
  (`parent.UserConstructionScript`))