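; BP_TuRretRed is the red turret variant, a child Blueprint that spawns red crystals and stops detecting pawns when the red gem count reaches zero.
; On BeginPlay it calls SpawnCrystals with RedCrystal.
; Every Tick, while PawnSensing is valid, it reads RedGems from player 0's BP_JonPlayerController and destroys that sensing component at zero.
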(event `self.ReceiveBeginPlay`
  (`self.SpawnCrystals` "/Game/machine_gun/CrystalBP/RedCrystal.RedCrystal_C"))

(event `self.ReceiveTick`
  (params (DeltaSeconds :type "Float (single-precision)"))
  (`/Engine/EditorBlueprintResources/StandardMacros.IsValid` (`self.PawnSensing`)
    (:`Is Valid`
      (bind _asbp_jon_player_controller (cast `/Game/Blueprints/MainCharacterBP´s/BP_JonPlayerController` (`GameplayStatics.GetPlayerController` 0)))
      (if (== (`/Game/Blueprints/MainCharacterBP´s/BP_JonPlayerController.RedGems` _asbp_jon_player_controller) 0)
        (`ActorComponent.K2_DestroyComponent` (`self.PawnSensing`))))))

(fn `UserConstructionScript`
  (`parent.UserConstructionScript`))