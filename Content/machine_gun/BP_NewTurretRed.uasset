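; BP_NewTurretRed is an enemy turret that shoots at the player and explodes once they hold enough red crystals.
; When PawnSensing sees BP_JonCharacter, it turns to face them, and a Delay paces bullet spawns from the Arrow, each with a shot sound.
; Tick polls the player's RedCrystalCount, triggering a one-time Niagara explosion, hiding the mesh and destroying the actor shortly after.
; A DestroyTurret event also allows immediate removal.
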(event `self.ReceiveTick`
  (params (DeltaSeconds :type "Float (single-precision)"))
  (bind _asbp_jon_character (cast `/Game/Blueprints/MainCharacterBP´s/BP_JonCharacter` (`GameplayStatics.GetPlayerCharacter` 0)))
  (if (>= (`/Game/Blueprints/MainCharacterBP´s/BP_JonCharacter.RedCrystalCount` _asbp_jon_character) 3)
    (`/Engine/EditorBlueprintResources/StandardMacros.DoOnce` false
      (:`Completed`
        (`NiagaraFunctionLibrary.SpawnSystemAtLocation` "/Game/VFX/NS_EXPLOSION.NS_EXPLOSION" (`SceneComponent.K2_GetComponentLocation` (`self.SkeletalMesh`)) (struct) (1.0 1.0 1.0) false)
        (`SceneComponent.SetVisibility` (`self.SkeletalMesh`) false false)
        (`ActorComponent.K2_DestroyComponent` (`self.Arrow`))
        (`KismetSystemLibrary.Delay` 0.5)
        (`self.K2_DestroyActor`)))))

(event `self.PawnSensing.OnSeePawn`
  (params (Pawn :type "Pawn Object Reference"))
  (cast `/Game/Blueprints/MainCharacterBP´s/BP_JonCharacter` Pawn)
  (`self.K2_SetActorRotation` (`KismetMathLibrary.FindLookAtRotation` (`self.K2_GetActorLocation`) (`self.K2_GetActorLocation` Pawn)))
  (`KismetSystemLibrary.Delay` 2.0)
  (`|SpawnActorFromClass` "/Game/machine_gun/BP_NewTurretBullet.BP_NewTurretBullet_C" (`SceneComponent.K2_GetComponentToWorld` (`self.Arrow`)) "Undefined" "MultiplyWithRoot" null null)
  (`FMODBlueprintStatics.PlayEventAtLocation` "/Game/FMOD/Events/Player_shoot_2.Player_shoot_2" (`SceneComponent.K2_GetComponentToWorld` (`self.Arrow`))))

(event `DestroyTurret`
  (`self.K2_DestroyActor`))

(fn `UserConstructionScript`)