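; BP_NewTurretBullet is a bullet actor, named for a turret, that damages the player character BP_JonCharacter on contact.
; When HitCollision begins an overlap, actors tagged Wall simply destroy the bullet.
; A hit on BP_JonCharacter applies fixed damage, spawns a blood Niagara effect, prints a scaled Shield value and destroys the bullet.
; Other actors are ignored, and the graph contains no movement logic.
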(event `self.HitCollision.OnComponentBeginOverlap`
  (params (OverlappedComponent :type "PrimitiveComponent Object Reference") (OtherActor :type "Actor Object Reference") (OtherComp :type "PrimitiveComponent Object Reference") (OtherBodyIndex :type Integer) (bFromSweep :type Boolean) (SweepResult :type "HitResult Structure (by ref)"))
  (if (`self.ActorHasTag` OtherActor "Wall")
    (`self.K2_DestroyActor`)
    (else
      (bind _asbp_jon_character (cast `/Game/Blueprints/MainCharacterBP´s/BP_JonCharacter` OtherActor))
      (`GameplayStatics.ApplyDamage` _asbp_jon_character 10.0)
      (`NiagaraFunctionLibrary.SpawnSystemAtLocation` "/Game/VFX/BLOOD_NIAGARA.BLOOD_NIAGARA" (`self.K2_GetActorLocation` _asbp_jon_character))
      (`KismetSystemLibrary.PrintString` (`KismetStringLibrary.Conv_DoubleToString` (* (`Jon.Shield` _asbp_jon_character) 10.0)))
      (`self.K2_DestroyActor`))))

(fn `UserConstructionScript`)