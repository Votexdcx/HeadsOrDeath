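; Turret actor that fires projectiles at the player and also holds crystal-spawning logic.
; When pawn sensing spots BP_JonCharacter, it turns to face the pawn, waits briefly, then spawns a projectile at the GunBarrel socket aimed at player 0's last movement-update location.
; SpawnCrystals waits a random delay, then spawns the given class at a random navmesh point around a fixed origin.
; A separate function decrements the crystal count.
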(event `self.PawnSensing.OnSeePawn`
  (params (Pawn :type "Pawn Object Reference"))
  (bind (_returnvalue_location _returnvalue_rotation _returnvalue_scale) (`KismetMathLibrary.BreakTransform` (`SceneComponent.GetSocketTransform` (`self.Turret`) "GunBarrel" "RTS_World")))
  (cast `/Game/Blueprints/MainCharacterBP´s/BP_JonCharacter` Pawn)
  (`self.K2_SetActorRotation` (`KismetMathLibrary.FindLookAtRotation` (`self.K2_GetActorLocation`) (`self.K2_GetActorLocation` Pawn)))
  (`KismetSystemLibrary.Delay` 0.5)
  (`|SpawnActorFromClass` "/Game/machine_gun/prjectile.prjectile_C" (`KismetMathLibrary.MakeTransform` _returnvalue_location (`KismetMathLibrary.Conv_VectorToRotator` (`KismetMathLibrary.Normal` (- (`CharacterMovementComponent.GetLastUpdateLocation` (`Character.CharacterMovement` (`GameplayStatics.GetPlayerCharacter` 0))) (`self.K2_GetActorLocation`)))) _returnvalue_scale) "Undefined" "MultiplyWithRoot" null null))

(event `SpawnCrystals`
  (params (CrysalClass :type "/Game/machine_gun/CrystalBP/Crystal Class Reference"))
  (`KismetSystemLibrary.Delay` (`KismetMathLibrary.RandomFloatInRange` 15.0 20.0))
  (bind _returnvalue (`GameplayStatics.GetActorOfClass` "/Script/NavigationSystem.RecastNavMesh"))
  (bind _output_get (set `self.location` (-682.064697 121.284319 -631.274208)))
  (bind _randomlocation (`NavigationSystemV1.K2_GetRandomLocationInNavigableRadius` _output_get 2000.0 _returnvalue "/Script/AIModule.NavFilter_AIControllerDefault"))
  (`|SpawnActorFromClass` CrysalClass (`KismetMathLibrary.Conv_VectorToTransform` _randomlocation) "AdjustIfPossibleButAlwaysSpawn" "MultiplyWithRoot" null null))

(fn `Subtractnumberofcrystals`
  (set `self.NumberOfCrystals` (- (`self.NumberOfCrystals`) 1)))

(fn `UserConstructionScript`)