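; BP_MeleeBot is a melee enemy with a health bar, a montage-based attack and a death that awards the player a point.
; Attack plays ATK_Montage, and its notify runs a forward sphere trace against Pawns to apply MeleeDamage.
; AnyDamage lowers Vida (health), which Tick pushes to the widget bar.
; At zero health the mesh ragdolls, then after a short delay BP_JonCharacter's Points increases and the bot is destroyed.
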(event `self.ReceiveTick`
  (params (DeltaSeconds :type "Float (single-precision)"))
  (bind _aswp_enemy_b1_health_bar (cast `/Game/Enemy_B1/WP_EnemyB1_HealthBar` (`WidgetComponent.GetWidget` (`self.HealthBarWidget`))))
  (`ProgressBar.SetPercent` (`/Game/Enemy_B1/WP_EnemyB1_HealthBar.EnemyB1HealthBar` _aswp_enemy_b1_health_bar) (/ (`self.Vida`) 40.0)))

(event `self.ReceiveAnyDamage`
  (params (Damage :type "Float (single-precision)") (DamageType :type "DamageType Object Reference") (InstigatedBy :type "Controller Object Reference") (DamageCauser :type "Actor Object Reference"))
  ;[1 1 1] Enemy Health
  (set `self.Vida` (- (`self.Vida`) Damage))
  (if (<= (`self.Vida`) 0.0)
    (`self.StopAnimMontage` "/Game/ENEMIES/MELEE/ATK_Montage.ATK_Montage")
    (`PrimitiveComponent.SetSimulatePhysics` (`self.Mesh`) true)
    (`KismetSystemLibrary.Delay` 0.7)
    (`|ExecutionSequence`
      (:`then_0`
        (bind _asbp_jon_character (cast `/Game/Blueprints/MainCharacterBP´s/BP_JonCharacter` (`GameplayStatics.GetPlayerCharacter` 0)))
        (`/Engine/EditorBlueprintResources/StandardMacros.IncrementInt` (`Jon.Points` _asbp_jon_character)))
      (:`then_1`
        (`self.K2_DestroyActor`)))))

(event `/Game/AI/BPI_AI.Attack`
  (bind _returnvalue (`self.K2_GetActorLocation`))
  (bind _meleedamage (`self.MeleeDamage`))
  (`|PlayMontage` (`self.Mesh`) "/Game/ENEMIES/MELEE/ATK_Montage.ATK_Montage"
    (:`OnNotifyBegin`
      (bind (_outhit _returnvalue_2) (`KismetSystemLibrary.SphereTraceSingleForObjects` _returnvalue (+ _returnvalue (* (`KismetMathLibrary.GetForwardVector` (`self.K2_GetActorRotation`)) 170.0)) 30.0 (`|MakeArray` "ObjectTypeQuery3" :!type "EObjectTypeQuery Enum")))
      (if _returnvalue_2
        (`GameplayStatics.ApplyDamage` (`.HitActor` (`GameplayStatics.BreakHitResult` _outhit)) _meleedamage)
        (`KismetSystemLibrary.PrintString` (`KismetStringLibrary.Conv_DoubleToString` _meleedamage))))))

(fn `UserConstructionScript`)