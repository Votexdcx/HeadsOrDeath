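; BP_CrawlerChase is a crawler enemy character that explodes on contact with the player character, BP_JonCharacter.
; A capsule hit applies radial damage with a debug sphere, then DEATH spawns explosion Niagara and sound before destroying the actor.
; Incoming damage lowers Vida and briefly swaps the face material.
; At zero health it shows a death face, enables mesh physics and stops movement, without calling DEATH.
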(event `DEATH`
  (bind _mesh (`self.Mesh`))
  (`NiagaraFunctionLibrary.SpawnSystemAtLocation` "/Game/ENEMIES/NS_EXPLOSION.NS_EXPLOSION" (`SceneComponent.K2_GetComponentLocation` _mesh) (struct) (1.0 1.0 1.0) false)
  (`FMODBlueprintStatics.PlayEventAtLocation` "/Game/FMOD/Events/Buff_Plus.Buff_Plus" (`SceneComponent.K2_GetComponentToWorld` _mesh))
  (`self.K2_DestroyActor`))

(event `self.ReceiveAnyDamage`
  (params (Damage :type "Float (single-precision)") (DamageType :type "DamageType Object Reference") (InstigatedBy :type "Controller Object Reference") (DamageCauser :type "Actor Object Reference"))
  (bind _mesh (`self.Mesh`))
  (`|ExecutionSequence`
    (:`then_0`
      (`FMODBlueprintStatics.PlayEvent2D` "/Game/FMOD/Events/Buff_Plus.Buff_Plus")
      (set `self.Vida` (- (`self.Vida`) Damage))
      (`PrimitiveComponent.SetMaterial` _mesh 2 "/Game/ENEMIES/MELEE/MAT_FACE_TAKE_DMG.MAT_FACE_TAKE_DMG")
      (`KismetSystemLibrary.Delay` 0.3)
      (`PrimitiveComponent.SetMaterial` _mesh 2 "/Game/ENEMIES/MELEE/FACE.FACE")
      (if (<= (`self.Vida`) 0.0)
        (`PrimitiveComponent.SetMaterial` _mesh 2 "/Game/ENEMIES/MELEE/MAT_FACE_DEATH.MAT_FACE_DEATH")
        (`PrimitiveComponent.SetSimulatePhysics` _mesh true)
        (`MovementComponent.StopMovementImmediately` (`self.CharacterMovement`))))))

(event `self.CapsuleComponent.OnComponentHit`
  (params (HitComponent :type "PrimitiveComponent Object Reference") (OtherActor :type "Actor Object Reference") (OtherComp :type "PrimitiveComponent Object Reference") (NormalImpulse :type "Vector Structure") (Hit :type "HitResult Structure (by ref)"))
  (cast `/Game/Blueprints/MainCharacterBP´s/BP_JonCharacter` OtherActor)
  (`GameplayStatics.ApplyRadialDamage` :`BaseDamage` 20.0 :`Origin` Hit_Location :`DamageRadius` 500.0 :`DamageCauser` self :`InstigatedByController` null)
  (`KismetSystemLibrary.PrintString` "RADIAL dmg")
  (`KismetSystemLibrary.DrawDebugSphere` (`self.K2_GetActorLocation`) 500.0)
  (`self.DEATH`))

(fn `UserConstructionScript`)