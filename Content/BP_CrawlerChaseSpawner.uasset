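; BP_CrawlerChaseSpawner is a spawner actor that keeps adding BP_CrawlerChase AI enemies to the level.
; After a random startup delay it plays a one-time particle effect at its billboard, then loops forever.
; Each loop spawns a crawler at a random reachable navmesh point within a wide radius of the spawner, then waits a random interval, with no spawn cap.
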(event `self.ReceiveBeginPlay`
  (`KismetSystemLibrary.Delay` (`KismetMathLibrary.RandomFloatInRange` 7.0 15.0))
  (`NiagaraFunctionLibrary.SpawnSystemAtLocation` null (`SceneComponent.K2_GetComponentLocation` (`self.Billboard`)))
  (`KismetSystemLibrary.Delay` 0.2)
  (`AIBlueprintHelperLibrary.SpawnAIFromClass` "/Game/AI/BP_CrawlerChase.BP_CrawlerChase_C" null (`NavigationSystemV1.K2_GetRandomReachablePointInRadius` (`self.K2_GetActorLocation`) 7000.0 null null) (struct) false null :!label _label)
  (`KismetSystemLibrary.RetriggerableDelay` (`KismetMathLibrary.RandomFloatInRange` 7.0 15.0))
  (goto _label))

(fn `UserConstructionScript`)