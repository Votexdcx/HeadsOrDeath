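; BP_EnemyCrawlerYellow is a crawler enemy that wanders, detects pawns and grants a buff to the player when killed.
; A self-repeating AIMoveTo requests short random moves, while PawnSensing sets the blackboard's hasSeenplayer flag.
; Lethal damage ragdolls the mesh, activates a buff through the player's BuffDebuffComponent and creates its widget.
; After a delay it destroys itself, first dealing radial damage that spares the player if IsEnemyExplodable is set.
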(event `self.ReceiveAnyDamage`
  (params (Damage :type "Float (single-precision)") (DamageType :type "DamageType Object Reference") (InstigatedBy :type "Controller Object Reference") (DamageCauser :type "Actor Object Reference"))
  (bind _returnvalue (`GameplayStatics.GetPlayerCharacter` 0))
  ;[1 1 1] Enemy Health
  (set `self.health` (- (`self.health`) Damage))
  (if (<= (`self.health`) 0.0)
    (`PrimitiveComponent.SetSimulatePhysics` (`self.Mesh`) true)
    (bind _asbp_jon_character (cast `/Game/Blueprints/MainCharacterBP´s/BP_JonCharacter` (`GameplayStatics.GetPlayerCharacter` 0)))
    (bind _returnvalue_2 (`BuffDebuffComponent.ActivateBuffPlus` (`/Game/Blueprints/MainCharacterBP´s/BP_JonCharacter.BuffDebuff Component` _asbp_jon_character)))
    (bind _asbp_jon_player_controller (cast `/Game/Blueprints/MainCharacterBP´s/BP_JonPlayerController` (`GameplayStatics.GetPlayerController` 0)))
    (`/Game/Blueprints/MainCharacterBP´s/BP_JonPlayerController.Create Buffs+ widget` _asbp_jon_player_controller _returnvalue_2)
    (`KismetSystemLibrary.Delay` 2.0)
    (bind _asbp_jon_character_2 (cast `/Game/Blueprints/MainCharacterBP´s/BP_JonCharacter` _returnvalue))
    (if (`BuffDebuffComponent.IsEnemyExplodable` (`/Game/Blueprints/MainCharacterBP´s/BP_JonCharacter.BuffDebuff Component` _asbp_jon_character_2))
      (`GameplayStatics.ApplyRadialDamage` 50.0 (`self.K2_GetActorLocation`) 300.0 "/Script/Engine.DamageType" (`|MakeArray` _returnvalue :!type "Actor Object Reference") self null))
    (`self.K2_DestroyActor`)))

(event `JumpToRandomLocation`
  ;[1 1 1] Budget AI
  (bind _randomlocation (`NavigationSystemV1.K2_GetRandomLocationInNavigableRadius` (`self.K2_GetActorLocation`) 40.0 null null))
  (`|AIMoveTo` null _randomlocation self
    (:`OnSuccess`
      (`self.JumpToRandomLocation`))))

(event `self.ReceiveBeginPlay`
  ;[1 1 1] Budget AI
  (`self.JumpToRandomLocation`))

(event `self.PawnSensing.OnSeePawn`
  (params (Pawn :type "Pawn Object Reference"))
  (`BlackboardComponent.SetValueAsBool` (`AIBlueprintHelperLibrary.GetBlackboard` (`AIBlueprintHelperLibrary.GetAIController` self)) "hasSeenplayer" true))

(fn `UserConstructionScript`)