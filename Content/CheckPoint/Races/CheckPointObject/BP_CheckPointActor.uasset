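; BP_CheckPointActor is a race checkpoint that the player collects by overlapping it.
; On overlap it confirms the other actor is the player's BP_JonCharacter, then destroys itself and plays a click sound.
; It switches on the character's current race, with identical branches for Race 1 and Race 2 that decrement the character's remaining checkpoint count.
; When that count reaches zero, it stops the character's stopwatch widget.
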(event `self.ReceiveActorBeginOverlap`
  (params (OtherActor :type "Actor Object Reference"))
  (bind _as_bp_jon_character (`self.As BP Jon Character`))
  (bind _as_bp_jon_character_2 (`self.As BP Jon Character`))
  (bind _numberofcheckpoints (`/Game/Blueprints/MainCharacterBP´s/BP_JonCharacter.NumberOfCheckPoints` _as_bp_jon_character))
  (bind _numberofcheckpoints_2 (`/Game/Blueprints/MainCharacterBP´s/BP_JonCharacter.NumberOfCheckPoints` _as_bp_jon_character_2))
  ;[1 1 1] Check if overlaping actor is player
  (bind _asbp_jon_character (cast `/Game/Blueprints/MainCharacterBP´s/BP_JonCharacter` (`GameplayStatics.GetPlayerPawn` 0)))
  (set `self.As BP Jon Character` _asbp_jon_character)
  (if (== OtherActor null)
    ;[1 1 1] Destroy Checkpoint with sound
    (`self.K2_DestroyActor`)
    (`GameplayStatics.PlaySound2D` "/Game/AdvancedLocomotionV4/Audio/UI/Click.Click" 1.0 1.0 0.0 null null)
    (switch `/Game/CheckPoint/Races/RaceList` (`/Game/Blueprints/MainCharacterBP´s/BP_JonCharacter.Race?` (`self.As BP Jon Character`))
      (:`NewEnumerator0`
        (set `/Game/Blueprints/MainCharacterBP´s/BP_JonCharacter.NumberOfCheckPoints` (- _numberofcheckpoints_2 1) _as_bp_jon_character_2)
        (if (== _numberofcheckpoints_2 0)
          (`/Game/CheckPoint/Races/StopWatchWidget.Stop Stop Watch` (`/Game/Blueprints/MainCharacterBP´s/BP_JonCharacter.StopWatchWidget` (`self.As BP Jon Character`)))))
      (:`NewEnumerator1`
        (set `/Game/Blueprints/MainCharacterBP´s/BP_JonCharacter.NumberOfCheckPoints` (- _numberofcheckpoints 1) _as_bp_jon_character)
        (if (== _numberofcheckpoints 0)
          (`/Game/CheckPoint/Races/StopWatchWidget.Stop Stop Watch` (`/Game/Blueprints/MainCharacterBP´s/BP_JonCharacter.StopWatchWidget` (`self.As BP Jon Character`))))))))

(fn `UserConstructionScript`)