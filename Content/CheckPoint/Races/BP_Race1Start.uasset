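; Race 1 start trigger that launches a timed checkpoint race when the player character overlaps it.
; On overlap it resets race state, disables input, shows a loading screen, spawns checkpoint actors and teleports the player.
; A delay loop polls the countdown widget, then restores input and starts the stopwatch.
; If another race state is active, it instead stops the stopwatch, destroys all checkpoints and briefly shows a failure widget.
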(event `self.ReceiveActorBeginOverlap`
  (params (OtherActor :type "Actor Object Reference"))
  (bind _as_bp_jon_character (`self.As BP Jon Character`))
  (bind _as_bp_jon_character_2 (`self.As BP Jon Character`))
  (bind _as_bp_jon_character_3 (`self.As BP Jon Character`))
  (bind _countdown_widget (`/Game/Blueprints/MainCharacterBP´s/BP_JonCharacter.CountDown Widget` (`self.As BP Jon Character`)))
  (bind _stopwatchwidget (`/Game/Blueprints/MainCharacterBP´s/BP_JonCharacter.StopWatchWidget` _as_bp_jon_character_3))
  ;[1 1 1] Check Overlaping Actor is Player
  (bind _asbp_jon_character (cast `/Game/Blueprints/MainCharacterBP´s/BP_JonCharacter` (`GameplayStatics.GetPlayerPawn` 0)))
  (bind _output_get (set `self.As BP Jon Character` _asbp_jon_character))
  (if (== _output_get OtherActor)
    ;[1 1 1] Check there is not a race already selected
    (if (`|EnumInequality` (`/Game/Blueprints/MainCharacterBP´s/BP_JonCharacter.Race?` (`self.As BP Jon Character`)) "NewEnumerator2")
      ;[1 1 1] Set Race Variables
      (set `/Game/Blueprints/MainCharacterBP´s/BP_JonCharacter.Race?` "NewEnumerator0" _as_bp_jon_character)
      (set `/Game/Blueprints/MainCharacterBP´s/BP_JonCharacter.NumberOfCheckPoints` 0 _as_bp_jon_character)
      ;[1 1 1] Disable Character Input
      (`self.DisableInput` (`self.As BP Jon Character`) (`GameplayStatics.GetPlayerController` 0))
      ;[1 1 1] Add Loading Screen
      (`KismetSystemLibrary.Delay` 0.2)
      (bind _returnvalue (`|CreateWidget` "/Game/CheckPoint/Races/LoadingWidget.LoadingWidget_C"))
      (`UserWidget.AddToViewport` _returnvalue 0)
      ;[1 1 1] Spawn Checkpoints
      (`|ExecutionSequence`
        (:`then_0`
          (`|SpawnActorFromClass` "/Game/CheckPoint/Races/CheckPointObject/BP_CheckPointActor.BP_CheckPointActor_C" (`KismetMathLibrary.MakeTransform` (-4062.0 -380.0 -200.0)) "Undefined" "MultiplyWithRoot" null null)
          (`self.K2_SetActorLocationAndRotation` _as_bp_jon_character_2 (4062.0 -380.0 -200.0) (struct :`Yaw` -90.0) false false)
          (`Controller.SetControlRotation` (`Pawn.GetController` _as_bp_jon_character_2) (`KismetMathLibrary.MakeRotator` 0.0 0.0 -90.0))
          (`KismetSystemLibrary.Delay` 0.2)
          (`Widget.RemoveFromParent` _returnvalue)
          (`UserWidget.AddToViewport` _countdown_widget 0)
          (`GameplayStatics.PlaySound2D` "/Game/AdvancedLocomotionV4/Audio/UI/Click.Click" 1.0 1.0 0.0 null null)
          (`/Game/CheckPoint/Races/CountDownWidget.Start Timer` _countdown_widget)
          (if (== (`/Game/CheckPoint/Races/CountDownWidget.Time` _countdown_widget) 0.0) :!label _label
            (`GameplayStatics.PlaySound2D` "/Engine/VREditor/Sounds/UI/Camera_Shutter.Camera_Shutter" 1.0 1.0 0.0 null null)
            (`self.EnableInput` _as_bp_jon_character_3 (`GameplayStatics.GetPlayerController` 0))
            (`UserWidget.AddToViewport` _stopwatchwidget 0)
            (`/Game/CheckPoint/Races/StopWatchWidget.Start Stop Watch` _stopwatchwidget)
            (else
              (`KismetSystemLibrary.Delay` 0.01)
              (goto _label))))
        (:`then_1`
          (`|SpawnActorFromClass` "/Game/CheckPoint/Races/CheckPointObject/BP_CheckPointActor.BP_CheckPointActor_C" (`KismetMathLibrary.MakeTransform` (-4062.0 -380.0 -200.0)) "Undefined" "MultiplyWithRoot" null null))
        (:`then_2`
          (`|SpawnActorFromClass` "/Game/CheckPoint/Races/CheckPointObject/BP_CheckPointActor.BP_CheckPointActor_C" (`KismetMathLibrary.MakeTransform` (-4062.0 -380.0 -200.0)) "Undefined" "MultiplyWithRoot" null null)))
      (else
        (set `/Game/Blueprints/MainCharacterBP´s/BP_JonCharacter.Race?` "NewEnumerator0" (`self.As BP Jon Character`))
        (`/Game/CheckPoint/Races/StopWatchWidget.Stop Stop Watch` (`/Game/Blueprints/MainCharacterBP´s/BP_JonCharacter.StopWatchWidget` (`self.As BP Jon Character`)))
        (bind _outactors (`GameplayStatics.GetAllActorsOfClass` "/Game/CheckPoint/Races/CheckPointObject/BP_CheckPointActor.BP_CheckPointActor_C"))
        (for _array_element _outactors
          (`self.K2_DestroyActor` _array_element))
        (bind _returnvalue_2 (`|CreateWidget` "/Game/CheckPoint/Races/FailedWidget.FailedWidget_C"))
        (`UserWidget.AddToViewport` _returnvalue_2 0)
        (`KismetSystemLibrary.Delay` 2.0)
        (`Widget.RemoveFromParent` _returnvalue_2)))))

(fn `UserConstructionScript`)