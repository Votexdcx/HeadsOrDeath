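; Enemy turret that turns to face the player character (BP_JonCharacter) when seen and fires projectiles from alternating barrels.
; PawnSensing sightings set the actor's yaw directly toward the pawn, then pass through a short Delay into a FlipFlop that alternates right and left shots.
; Each shot spawns EnemyProjectile at its arrow component, plays a shoot montage and activates that side's muzzle flash.
; Montage names are opposite to the firing side.
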(event `self.PawnSensing.OnSeePawn`
  (params (Pawn :type "Pawn Object Reference"))
  (bind (_returnvalue_roll _returnvalue_pitch _returnvalue_yaw) (`KismetMathLibrary.BreakRotator` (`KismetMathLibrary.FindLookAtRotation` (`self.K2_GetActorLocation`) (`self.K2_GetActorLocation` Pawn))))
  (cast `/Game/Blueprints/MainCharacterBP´s/BP_JonCharacter` Pawn)
  (`self.K2_SetActorRotation` (`KismetMathLibrary.MakeRotator` 0.0 0.0 _returnvalue_yaw))
  (`KismetSystemLibrary.Delay` 0.2)
  (`/Engine/EditorBlueprintResources/StandardMacros.FlipFlop`
    (:`A`
      (`self.Shoot Right`))
    (:`B`
      (`self.Shoot Left`))))

(event `Shoot Right`
  (`|SpawnActorFromClass` "/Game/Enemy_B1/EnemyProjectile.EnemyProjectile_C" (`SceneComponent.K2_GetComponentToWorld` (`self.Arrow1`)) "Undefined" "MultiplyWithRoot" null null)
  (`|PlayMontage` (`self.SkeletalMesh`) "/Game/ENEMIES/TURRET/SHOOT_LEFT_MONTAGE.SHOOT_LEFT_MONTAGE"
    (:`then`
      (`ActorComponent.Activate` (`self.MUZZLE_FLASH_R`) true))))

(event `Shoot Left`
  (`|SpawnActorFromClass` "/Game/Enemy_B1/EnemyProjectile.EnemyProjectile_C" (`SceneComponent.K2_GetComponentToWorld` (`self.Arrow`)) "Undefined" "MultiplyWithRoot" null null)
  (`|PlayMontage` (`self.SkeletalMesh`) "/Game/ENEMIES/TURRET/SHOOT_RIGHT_MONTAGE.SHOOT_RIGHT_MONTAGE"
    (:`then`
      (`ActorComponent.Activate` (`self.MUZZLE_FLASH_L`) true))))

(fn `UserConstructionScript`)